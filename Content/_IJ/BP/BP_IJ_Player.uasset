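; Player character Blueprint that handles attack-facing rotation, target lock-on and the HP bar widget.
; Left click uses a timeline to turn the actor's yaw toward control rotation, outside side view and kill montages.
; BeginPlay initializes the TS targeting component with AI Perception; T locks on and Q/E switch targets left or right.
; Disconnected leftovers cover camera blending, android bot aiming and interaction montages; Tick and CameraMove are empty.
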(event `Key|LeftMouseButton`
  (params (Key :type "Key Structure"))
  ;[1 1 1] 러프러프
  (:`Pressed`
    (if (`self.bIsSideView`)
      _
      (elif (not (`IJ_PlayerMovement.bIsKillMontage` (`self.playerMovement`)))
        (bind (_direction _alpha) (`Timeline|Timeline_0` :!via `PlayFromStart`)
          (:`Update`
            (bind (_returnvalue_roll _returnvalue_pitch _returnvalue_yaw) (`KismetMathLibrary.BreakRotator` (`KismetMathLibrary.RLerp` (`self.K2_GetActorRotation`) (`self.GetControlRotation`) _alpha true)))
            (`self.K2_SetActorRotation` (`KismetMathLibrary.MakeRotator` 0.0 0.0 _returnvalue_yaw))))))))

(event `self.ReceiveBeginPlay`
  (`/Game/TheTargetingSystem/_Component/TS.Initialize Variables` (`self.TS`) (`self.AIPerception`) self)
  (bind _returnvalue (`|CreateWidget` "/Game/YS/YS_Blueprint/Widget/YS_WBP_PlayerHpBar.YS_WBP_PlayerHpBar_C" (`GameplayStatics.GetPlayerController` 0)))
  (`UserWidget.AddToViewport` _returnvalue 0))

(event `CameraMove`
  ;[1 1 1] 러프러프
)

(event `Key|T`
  (params (Key :type "Key Structure"))
  (:`Pressed`
    (`/Game/TheTargetingSystem/_Component/TS.Lock On To Target` (`self.TS`))
    (`KismetSystemLibrary.PrintString` "Hello")))

(event `Key|Q`
  (params (Key :type "Key Structure"))
  (:`Pressed`
    (`/Game/TheTargetingSystem/_Component/TS.Lock On To Target To The Left` (`self.TS`))))

(event `Key|E`
  (params (Key :type "Key Structure"))
  (:`Pressed`
    (`/Game/TheTargetingSystem/_Component/TS.Lock On To Target To The Right` (`self.TS`))))

(event `Key|V`
  (params (Key :type "Key Structure")))

(event `self.ReceiveTick`
  (params (DeltaSeconds :type "Float (single-precision)")))

(fn `UserConstructionScript`)