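; BP_Chain is a construction-time actor that lays copies of a static mesh along a spline, by its name to form a chain.
; The construction script creates an instanced static mesh component and adds instances at Spacing intervals over the spline's length, each following the spline's local location and rotation.
; Size sets the relative scale of both the spline and instance component, redundantly inside the loop.
; The event graph has no active logic.
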(fn `UserConstructionScript`
  (bind _spline (`self.Spline`))
  (bind _spacing (`self.Spacing`))
  (bind _returnvalue (`AddComponent|NODE_AddInstancedStaticMeshComponent-4`))
  (`StaticMeshComponent.SetStaticMesh` _returnvalue (`self.Static Mesh`))
  (set `self.Local Instance mesh` _returnvalue)
  (`InstancedStaticMeshComponent.ClearInstances` (`self.Local Instance mesh`))
  ;[1 1 1] Comment
  (for _index (range (+ (`.ReturnValue` (`KismetMathLibrary.FMod` (`SplineComponent.GetSplineLength` _spline) _spacing)) 1))
    (bind _returnvalue_2 (* _index _spacing))
    (`InstancedStaticMeshComponent.AddInstance` (`self.Local Instance mesh`) (`KismetMathLibrary.MakeTransform` (`SplineComponent.GetLocationAtDistanceAlongSpline` _spline _returnvalue_2 "Local") (`SplineComponent.GetRotationAtDistanceAlongSpline` _spline _returnvalue_2 "Local")))
    (`SceneComponent.SetRelativeScale3D` _spline (`KismetMathLibrary.Conv_DoubleToVector` (`self.Size`)))
    (`SceneComponent.SetRelativeScale3D` (`self.Local Instance mesh`) (`KismetMathLibrary.Conv_DoubleToVector` (`self.Size`)))))