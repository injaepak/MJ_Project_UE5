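; BP_Traffic animates a looping stream of cars along a spline using hierarchical instanced mesh instances.
; The construction script spaces CarCount instances evenly along the spline and applies the material.
; Tick adds a shared wrapping Timer to each start offset, then updates transforms from spline distance with zero pitch and flipped yaw.
; Timer advances by DeltaSeconds/TrafficSpeed per car inside the loop, so speed depends on car count.
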(event `self.ReceiveBeginPlay`)

(event `self.ReceiveTick`
  (params (DeltaSeconds :type "Float (single-precision)"))
  (bind _spline (`self.Spline`))
  ;[1 1 1] Calculate the dynamic position of the instance along the spline
  (`|ExecutionSequence`
    (:`then_0`
      (for (_array_element _array_index) (`self.Start Position`)
        (bind _output_get (set `self.timer` (+ (stale _output_get) (/ DeltaSeconds (`self.TrafficSpeed`)))))
        ;;[1 1 1] When the timer comes to 1 reset it
        (`/Engine/EditorBlueprintResources/StandardMacros.CompareFloat` _output_get 1.0
          (:`>`
            (set `self.timer` 0.0 :!label _label))
          (:`==`
            (goto _label))
          (:`<`
            _))
        (bind _returnvalue (+ _array_element _output_get))
        (`KismetArrayLibrary.Array_Set` (`self.instance position along spline`) _array_index _returnvalue)
        ;;[1 1 1] When the position of the instance comes to the end of the spline (1) we transfer it to the Star Spline (0)
        (`/Engine/EditorBlueprintResources/StandardMacros.CompareFloat` _returnvalue 1.0
          (:`>`
            _)
          (:`==`
            _))
        (`KismetArrayLibrary.Array_Set` (`self.instance position along spline`) _array_index (- _returnvalue 1.0))))
    (:`then_1`
      ;[1 1 1] update positions for instances
      (for (_array_element_2 _array_index_2) (`self.instance position along spline`)
        (bind _returnvalue_2 (`KismetMathLibrary.Lerp` 0.0 (`SplineComponent.GetSplineLength` _spline) _array_element_2))
        (`InstancedStaticMeshComponent.UpdateInstanceTransform` (`self.Instance_0`) _array_index_2 (`KismetMathLibrary.MakeTransform` (`SplineComponent.GetLocationAtDistanceAlongSpline` _spline _returnvalue_2 "Local") (`KismetMathLibrary.MakeRotator` (.roll (`SplineComponent.GetRotationAtDistanceAlongSpline` _spline _returnvalue_2 "Local")) 0.0 (+ (.yaw (`SplineComponent.GetRotationAtDistanceAlongSpline` _spline _returnvalue_2 "Local")) 180.0))) false false false)))))

(fn `UserConstructionScript`
  (locals (NewLocalVar_0 :type "MaterialInterface Object Reference"))
  (bind _start_position (`self.Start Position`))
  (bind _spline (`self.Spline`))
  (bind _car_count (`self.Car count`))
  (`|ExecutionSequence`
    (:`then_0`
      ;[1 1 1] Clean arrays
      (`KismetArrayLibrary.Array_Clear` (`self.Start Position`))
      (`KismetArrayLibrary.Array_Clear` (`self.instance position along spline`))
      (bind _returnvalue (`AddComponent|NODE_AddHierarchicalInstancedStaticMeshComponent-0`))
      (set `self.Instance_0` _returnvalue)
      ;[1 1 1] We set the starting positions for instances (1 divide on the number of instances)
      (for _index (range 1 (+ _car_count 1))
        (`KismetArrayLibrary.Array_Add` (`self.instance position along spline`))
        (bind _returnvalue_2 (`KismetArrayLibrary.Array_Add` _start_position (* (- _index 1) (/ 1.0 (`KismetMathLibrary.Conv_IntToDouble` _car_count)))))
        (bind _returnvalue_3 (`KismetMathLibrary.Lerp` 0.0 (`SplineComponent.GetSplineLength` _spline) (`|GetArrayItem` _start_position _returnvalue_2)))
        ;[1 1 1] We put instances on the position along the spline (0 beginning of the spline, 1 end of the spline)
        (`InstancedStaticMeshComponent.AddInstance` (`self.Instance_0`) (`KismetMathLibrary.MakeTransform` (`SplineComponent.GetLocationAtDistanceAlongSpline` _spline _returnvalue_3 "Local") (`KismetMathLibrary.MakeRotator` (.roll (`SplineComponent.GetRotationAtDistanceAlongSpline` _spline _returnvalue_3 "Local")) 0.0 (+ (.yaw (`SplineComponent.GetRotationAtDistanceAlongSpline` _spline _returnvalue_3 "Local")) 180.0))))))
    (:`then_1`
      (`PrimitiveComponent.SetMaterial` (`self.Instance_0`) 0 (`self.Material`)))))