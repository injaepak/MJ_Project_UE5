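; BP_WaterObj is a floating water prop that bobs, rocks and spins a configurable mesh, Buoy01.
; Construction applies the base rotation, mesh and material.
; Each Tick adds constant yaw, then chains three flag-driven ping-pong counters for vertical movement, roll and pitch, skipping downstream steps when one reverses.
; The counters drive per-frame world deltas, with Lerp between positive and negative rotation rates, unscaled by delta time.
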(event `self.ReceiveTick`
  (params (DeltaSeconds :type "Float (single-precision)"))
  (bind _buoy01 (`self.Buoy01`))
  (bind _rotation_x (`self.Rotation X`))
  (bind _float_var_2 (`self.Float Var 2`))
  (bind _rotation_x_speed (`self.Rotation X Speed`))
  (bind _movespeed (`self.MoveSpeed`))
  (bind _rotation_y_speed (`self.Rotation Y Speed`))
  (bind _float_var_3 (`self.Float Var 3`))
  (bind _rotation_y (`self.Rotation Y`))
  (bind _float_var_1 (`self.Float Var 1`))
  (bind _float_var_1_2 (`self.Float Var 1`))
  (bind _move (`self.Move`))
  (`SceneComponent.K2_AddWorldRotation` _buoy01 (`KismetMathLibrary.MakeRotator` 0.0 0.0 (`self.Rotation Z Speed`)) false false)
  (if (`self.Boolean Var 1`)
    (`/Engine/EditorBlueprintResources/StandardMacros.CompareFloat` _float_var_1_2 _move
      (:`>`
        (set `self.Boolean Var 1` false))
      (:`==`
        (set `self.Float Var 1` (+ _float_var_1_2 _movespeed) :!label _label)
        (`SceneComponent.K2_AddWorldTransform` _buoy01 (`KismetMathLibrary.Conv_VectorToTransform` (* (0.0 0.0 1.0) (`self.Float Var 1`))) false false :!label _label_2)
        (if (`self.Boolean Var 2`)
          (`/Engine/EditorBlueprintResources/StandardMacros.CompareFloat` _float_var_2 1.0
            (:`>`
              (set `self.Boolean Var 2` false))
            (:`==`
              (set `self.Float Var 2` (+ _float_var_2 _rotation_x_speed) :!label _label_3)
              (`SceneComponent.K2_AddWorldRotation` (`self.Buoy01`) (`KismetMathLibrary.MakeRotator` (`KismetMathLibrary.Lerp` _rotation_x (* _rotation_x -1.0) _float_var_2)) false false :!label _label_4)
              (if (`self.Boolean Var 3`)
                (`/Engine/EditorBlueprintResources/StandardMacros.CompareFloat` _float_var_3 1.0
                  (:`>`
                    (set `self.Boolean Var 3` false))
                  (:`==`
                    (set `self.Float Var 3` (+ _float_var_3 _rotation_y_speed) :!label _label_5)
                    (`SceneComponent.K2_AddWorldRotation` (`self.Buoy01`) (`KismetMathLibrary.MakeRotator` 0.0 (`KismetMathLibrary.Lerp` _rotation_y (* _rotation_y -1.0) _float_var_3)) false false :!label _label_6))
                  (:`<`
                    (goto _label_5)))
                (else
                  (`/Engine/EditorBlueprintResources/StandardMacros.CompareFloat` _float_var_3
                    (:`>`
                      (set `self.Float Var 3` (- _float_var_3 _rotation_y_speed) :!label _label_7)
                      (goto _label_6))
                    (:`==`
                      (goto _label_7))
                    (:`<`
                      (set `self.Boolean Var 3` true))))))
            (:`<`
              (goto _label_3)))
          (else
            (`/Engine/EditorBlueprintResources/StandardMacros.CompareFloat` _float_var_2
              (:`>`
                (set `self.Float Var 2` (- _float_var_2 _rotation_x_speed) :!label _label_8)
                (goto _label_4))
              (:`==`
                (goto _label_8))
              (:`<`
                (set `self.Boolean Var 2` true))))))
      (:`<`
        (goto _label)))
    (else
      (`/Engine/EditorBlueprintResources/StandardMacros.CompareFloat` _float_var_1 (* _move -1.0)
        (:`>`
          (set `self.Float Var 1` (- _float_var_1 _movespeed) :!label _label_9)
          (goto _label_2))
        (:`==`
          (goto _label_9))
        (:`<`
          (set `self.Boolean Var 1` true))))))

(fn `UserConstructionScript`
  (bind _buoy01 (`self.Buoy01`))
  (`SceneComponent.K2_SetRelativeRotation` _buoy01 (`self.base rotation`) false false)
  (`StaticMeshComponent.SetStaticMesh` _buoy01 (`self.Mesh`))
  (`PrimitiveComponent.SetMaterial` _buoy01 0 (`self.Material`)))