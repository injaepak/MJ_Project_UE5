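; Spline-driven wire prop that builds spline meshes along its Spline in the construction script.
; SplineMeshVar picks the layout: one segment per spline point pair using point tangents, or segments at fixed Spacing along the length with directions scaled by TangentScale.
; Each segment's component variant comes from WireVar, then both layouts share uniform WireSize scaling and a dynamic material instance chosen by MaterialVar.
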(fn `UserConstructionScript`
  (bind _conponent_1 (`self.Conponent 1`))
  (bind _spline (`self.Spline`))
  (bind _spline_2 (`self.Spline`))
  (bind _wire_size (`self.Wire Size`))
  (bind _points (`self.Points`))
  (bind _spacing (`self.Spacing`))
  (bind _tangent_scale (`self.Tangent Scale`))
  (bind _conponent_1_2 (`self.Conponent 1`))
  (bind (_location _tangent) (`SplineComponent.GetLocationAndTangentAtSplinePoint` _spline _points "Local"))
  (bind (_location_2 _tangent_2) (`SplineComponent.GetLocationAndTangentAtSplinePoint` _spline (+ _points 1) "Local"))
  (set `self.Conponent 1` null)
  (switch `int` (`self.Spline Mesh Var`)
    (:`Default`
      (for _index (range (+ (- (`SplineComponent.GetNumberOfSplinePoints` (`self.Spline`)) 2) 1)) :!label _label
        (set `self.Points` _index)
        (switch `int` (`self.Wire Var`)
          (:`Default`
            (bind _returnvalue (`AddComponent|NODE_AddSplineMeshComponent-13` :!label _label_2))
            (set `self.Conponent 1` _returnvalue))
          (:`0`
            (goto _label_2))
          (:`1`
            (bind _returnvalue_2 (`AddComponent|NODE_AddSplineMeshComponent-1`))
            (set `self.Conponent 1` _returnvalue_2))
          (:`2`
            (bind _returnvalue_3 (`AddComponent|NODE_AddSplineMeshComponent-2`))
            (set `self.Conponent 1` _returnvalue_3))
          (:`3`
            (bind _returnvalue_4 (`AddComponent|NODE_AddSplineMeshComponent-7`))
            (set `self.Conponent 1` _returnvalue_4))
          (:`4`
            (bind _returnvalue_5 (`AddComponent|NODE_AddSplineMeshComponent-8`))
            (set `self.Conponent 1` _returnvalue_5))
          (:`5`
            (bind _returnvalue_6 (`AddComponent|NODE_AddSplineMeshComponent-9`))
            (set `self.Conponent 1` _returnvalue_6))
          (:`6`
            (bind _returnvalue_7 (`AddComponent|NODE_AddSplineMeshComponent-15`))
            (set `self.Conponent 1` _returnvalue_7)))
        (`SplineMeshComponent.SetStartAndEnd` _conponent_1 _location _tangent _location_2 _tangent_2 true)
        (`SplineMeshComponent.SetStartScale` _conponent_1 (`KismetMathLibrary.MakeVector2D` _wire_size _wire_size) true :!label _label_3)
        (`SplineMeshComponent.SetEndScale` _conponent_1 (`KismetMathLibrary.MakeVector2D` _wire_size _wire_size) true)
        (switch `int` (`self.Material Var`)
          (:`Default`
            (bind _returnvalue_8 (`KismetMaterialLibrary.CreateDynamicMaterialInstance` "/Game/NeonCity/Materials/Props/MI_Wire01.MI_Wire01" :!label _label_4))
            (`PrimitiveComponent.SetMaterial` _conponent_1_2 0 _returnvalue_8))
          (:`0`
            (goto _label_4))
          (:`1`
            (bind _returnvalue_9 (`KismetMaterialLibrary.CreateDynamicMaterialInstance` "/Game/NeonCity/Materials/Props/MI_Wire02.MI_Wire02"))
            (`PrimitiveComponent.SetMaterial` _conponent_1_2 0 _returnvalue_9))
          (:`2`
            (bind _returnvalue_10 (`KismetMaterialLibrary.CreateDynamicMaterialInstance` "/Game/NeonCity/Materials/Props/MI_Wire03.MI_Wire03"))
            (`PrimitiveComponent.SetMaterial` _conponent_1_2 0 _returnvalue_10))
          (:`3`
            (bind _returnvalue_11 (`KismetMaterialLibrary.CreateDynamicMaterialInstance` "/Game/NeonCity/Materials/Props/MI_Wire04.MI_Wire04"))
            (`PrimitiveComponent.SetMaterial` _conponent_1_2 0 _returnvalue_11))
          (:`4`
            (bind _returnvalue_12 (`KismetMaterialLibrary.CreateDynamicMaterialInstance` "/Game/NeonCity/Materials/Props/MI_Wire05.MI_Wire05"))
            (`PrimitiveComponent.SetMaterial` _conponent_1_2 0 _returnvalue_12)))))
    (:`0`
      (goto _label))
    (:`1`
      (for _index_2 (range (+ (`.ReturnValue` (`KismetMathLibrary.FMod` (`SplineComponent.GetSplineLength` _spline_2) _spacing)) 1))
        (switch `int` (`self.Wire Var`)
          (:`Default`
            (bind _returnvalue_13 (`AddComponent|NODE_AddSplineMeshComponent-4` :!label _label_5))
            (set `self.Conponent 1` _returnvalue_13))
          (:`0`
            (goto _label_5))
          (:`1`
            (bind _returnvalue_14 (`AddComponent|NODE_AddSplineMeshComponent-5`))
            (set `self.Conponent 1` _returnvalue_14))
          (:`2`
            (bind _returnvalue_15 (`AddComponent|NODE_AddSplineMeshComponent-6`))
            (set `self.Conponent 1` _returnvalue_15))
          (:`3`
            (bind _returnvalue_16 (`AddComponent|NODE_AddSplineMeshComponent-10`))
            (set `self.Conponent 1` _returnvalue_16))
          (:`4`
            (bind _returnvalue_17 (`AddComponent|NODE_AddSplineMeshComponent-11`))
            (set `self.Conponent 1` _returnvalue_17))
          (:`5`
            (bind _returnvalue_18 (`AddComponent|NODE_AddSplineMeshComponent-12`))
            (set `self.Conponent 1` _returnvalue_18))
          (:`6`
            (bind _returnvalue_19 (`AddComponent|NODE_AddSplineMeshComponent-14`))
            (set `self.Conponent 1` _returnvalue_19)))
        (bind _returnvalue_20 (* _index_2 _spacing))
        (bind _returnvalue_21 (+ _returnvalue_20 _spacing))
        (`SplineMeshComponent.SetStartAndEnd` _conponent_1 (`SplineComponent.GetLocationAtDistanceAlongSpline` _spline_2 _returnvalue_20 "Local") (* (`SplineComponent.GetDirectionAtDistanceAlongSpline` _spline_2 _returnvalue_20 "Local") _tangent_scale) (`SplineComponent.GetLocationAtDistanceAlongSpline` _spline_2 _returnvalue_21 "Local") (* (`SplineComponent.GetDirectionAtDistanceAlongSpline` _spline_2 _returnvalue_21 "Local") _tangent_scale) true)
        (goto _label_3)))))