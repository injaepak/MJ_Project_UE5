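; BP_HangingWires is a construction-script prop that builds a bundle of hanging wires from three sets of instanced static meshes.
; It generates one transform per mesh, offset by StartY and StartZ, aimed along End, with length scaled from End's summed components and randomized cross-scale.
; Enabling Freeze skips regeneration and reuses the stored transforms, preserving the random layout.
; The transform array is split sequentially across the three instanced components by their mesh counts.
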(fn `UserConstructionScript`
  (bind _number_of_meshes1 (`self.number of meshes1`))
  (bind _transform (`self.Transform`))
  (bind (_yaw _pitch) (`KismetMathLibrary.GetYawPitchFromVector` (`self.End`)))
  (bind _returnvalue (+ _number_of_meshes1 (`self.number of meshes2`)))
  (`|ExecutionSequence`
    (:`then_0`
      (if (not (`self.Freeze`))
        (`KismetArrayLibrary.Array_Clear` (`self.Transform`))
        (for _ (range (+ (+ (`self.number of meshes1`) (`self.number of meshes2`)) (`self.number of meshes3`)))
          (`KismetArrayLibrary.Array_Add` (`self.Transform`) (`KismetMathLibrary.MakeTransform` (`KismetMathLibrary.MakeVector` 0.0 (`KismetMathLibrary.RandomFloatInRange` (.y (`self.Start_Y-`)) (.y (`self.Start_Y+`))) (`KismetMathLibrary.RandomFloatInRange` (.z (`self.Start_Z-`)) (.z (`self.Start_Z+`)))) (`KismetMathLibrary.MakeRotator` 0.0 _pitch _yaw) (`KismetMathLibrary.MakeVector` (/ (+ (+ (.x (`self.End`)) (.y (`self.End`))) (.z (`self.End`))) (`self.MeshScaleDivide`)) (`KismetMathLibrary.RandomFloatInRange` 0.8 1.2) (`KismetMathLibrary.RandomFloatInRange` 0.8 2.0))))))
      (bind _returnvalue_2 (`AddComponent|NODE_AddInstancedStaticMeshComponent-3`))
      (set `self.Instance Meshes` _returnvalue_2)
      (bind _returnvalue_3 (`AddComponent|NODE_AddInstancedStaticMeshComponent-4`))
      (set `self.Instance Meshes2` _returnvalue_3)
      (bind _returnvalue_4 (`AddComponent|NODE_AddInstancedStaticMeshComponent-5`))
      (set `self.Instance Meshes3` _returnvalue_4)
      (for _index (range _number_of_meshes1)
        (set `self.number of meshes3_0` _index)
        (`InstancedStaticMeshComponent.AddInstance` (`self.Instance Meshes`) (`|GetArrayItem` _transform _index)))
      (for _index_2 (range _number_of_meshes1 _returnvalue)
        (`InstancedStaticMeshComponent.AddInstance` (`self.Instance Meshes2`) (`|GetArrayItem` _transform _index_2)))
      (for _index_3 (range _returnvalue (+ _returnvalue (`self.number of meshes3`)))
        (`InstancedStaticMeshComponent.AddInstance` (`self.Instance Meshes3`) (`|GetArrayItem` _transform _index_3))))))